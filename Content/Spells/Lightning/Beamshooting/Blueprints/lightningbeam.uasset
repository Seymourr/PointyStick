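; Lightning beam spell actor that fires a lightning laser forward and destroys Imp enemies it hits.
; Each Tick shows the beam, plays its sound and runs a multi line trace along the emitter's forward vector.
; Each hit moves the beam target and spawns a hit effect, and Imps get an impulse before destruction.
; BeamCharge counts to ten, clearing the emitter template until its timer stops, though Tick never reads the count.
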(event `self.ReceiveTick`
  (params (DeltaSeconds :type "Float (single-precision)"))
  (bind _laseremitter (`self.LaserEmitter`))
  (bind _laseremitter_2 (`self.LaserEmitter`))
  (bind _laseremitter_3 (`self.LaserEmitter`))
  (bind _returnvalue (`SceneComponent.K2_GetComponentLocation` _laseremitter))
  ;[1 1 1] use to check if the beam is charged enough
  ;[1 1 1] if beam is charged enough then it will appear, if not it will not appear
  (`ParticleSystemComponent.SetTemplate` _laseremitter_3 "/Game/Spells/Lightning/Beamshooting/particles/lightning_beam_shoot.lightning_beam_shoot")
  (`SceneComponent.SetVisibility` _laseremitter_3 true true)
  (`GameplayStatics.PlaySoundAtLocation` "/Game/Sounds/lightning_loose_1.lightning_loose_1")
  (bind _outhits (`KismetSystemLibrary.LineTraceMulti_NEW` _returnvalue (+ _returnvalue (* (`SceneComponent.GetForwardVector` _laseremitter) 5000.0)) "TraceTypeQuery1"))
  (for _array_element _outhits
    (bind (_bblockinghit _binitialoverlap _time _location _impactpoint _normal _impactnormal _physmat _hitactor) (`GameplayStatics.BreakHitResult` _array_element))
    ;[1 1 1] set the beam source and target point and update these point
    (bind _output_get (set `self.LaserTarget` _location))
    (`ParticleSystemComponent.SetBeamSourcePoint` _laseremitter_2 0 (0.0 0.0 0.0) 0)
    (`ParticleSystemComponent.SetBeamTargetPoint` _laseremitter_2 0 _output_get 0)
    ;[1 1 1] set the hit point in the location of target point
    (`GameplayStatics.SpawnEmitterAtLocation` "/Game/Spells/Lightning/Beamshooting/particles/lightning_hit.lightning_hit" _output_get)
    (bind _asenemy_imp (cast `/Game/Monsters/EnemyImp` _hitactor))
    (`PrimitiveComponent.AddImpulseAtLocation` (`/Game/Monsters/EnemyImp.SkeletalMesh` _asenemy_imp) (750.0 750.0 750.0) _output_get "None")
    (`self.K2_DestroyActor` _asenemy_imp)))

(fn `BeamCharge`
  (bind _intbeamchargerate (`self.IntBeamChargeRate`))
  (set `self.IntBeamChargeRate` (+ _intbeamchargerate 1))
  (if (== _intbeamchargerate 10)
    (`KismetSystemLibrary.K2_ClearTimer` null "BeamCharge")
    (else
      (`ParticleSystemComponent.SetTemplate` (`self.LaserEmitter`) null))))

(fn `UserConstructionScript`)